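; Main game mode that runs endless, escalating waves of mobs through the level's BP_MobSpawner actors.
; Each wave grows the pool and concurrent cap with the wave number, unhides sniper pickups, and queues mobs on random spawners up to the cap.
; OnMobDefeated queues replacements while enough mobs remain, then starts a timer for the next wave once none are left.
; The pool is count-only in practice, as GetMobFromPool always returns BP_Mob.
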(event EventBeginPlay
  (CallFunction|GetSpawners)
  (CallFunction|BeginNewWave))

(event EventTick
  (params (DeltaSeconds :type Float%20%28single-precision%29)))

(fn ConstructionScript)

(fn GetSpawners
  (bind _outactors (Actor|GetAllActorsOfClass "/Game/MainGameFiles/Characters/Mobs/BP_MobSpawner.BP_MobSpawner_C"))
  (Variables|Default|SetMobSpawners _outactors))

(fn WaveStart
  (CallFunction|BuildMobPool)
  (for _index (range 0 (- (Math|Integer|Min(Integer) (CallFunction|GetMobPoolSize) (Variables|Default|GetMobMaxCount)) 1))
    (bind _mob_ (CallFunction|GetMobfromPool))
    (Default|AddMobtoQueue (.OutItem (Utilities|Array|Random (Variables|Default|GetMobSpawners))) _mob_)))

(fn TransitionEntered
  (params (Time%20Transition :type Float%20%28single-precision%29))
  (bind _returnvalue (Utilities|Time|SetTimerbyFunctionName 0 "BeginNewWave" Time%20Transition))
  (Variables|Default|SetTransition%20Timer _returnvalue))

(fn BuildMobPool
  (Variables|Default|SetMobsRemaining (CallFunction|GetMobPoolSize)))

(fn BeginNewWave
  (bind _result (Math|Integer|IncrementInt (Variables|Default|GetWaveNumber))
    (:%20%20
      (Variables|Default|SetWaveNumber _result)
      (Variables|Default|SetMobsRemaining (+ (Variables|Default|GetDefaultMobRemain) (Variables|Default|GetWaveNumber)))
      (Variables|Default|SetMobMaxCount (+ (Variables|Default|GetDefaultMobCount) (Variables|Default|GetWaveNumber)))
      (Utilities|Map|Add (Variables|Default|GetMobsPool) "/Game/MainGameFiles/Characters/Mobs/BP_Mob.BP_Mob_C" (+ (Variables|Default|GetWaveNumber) (.Value (Utilities|Map|Find (Variables|Default|GetDefaultMobPool) "/Game/MainGameFiles/Characters/Mobs/BP_MobSpawner.BP_MobSpawner_C"))))
      (Development|PrintString (Utilities|String|ToString(Integer) (.Value (Utilities|Map|Find (Variables|Default|GetMobsPool) "/Game/MainGameFiles/Characters/Mobs/BP_Mob.BP_Mob_C"))))
      (bind _outactors (Actor|GetAllActorsOfClass "/Game/MainGameFiles/Weapons/BP_SniperPickUp.BP_SniperPickUp_C"))
      (for _array_element _outactors
        (Rendering|SetActorHiddenInGame _array_element false))
      (CallFunction|WaveStart))))

(fn OnMobDefeated
  (bind _result (Math|Integer|DecrementInt (Variables|Default|GetMobsRemaining))
    (:%20%20
      (if (< _result (Variables|Default|GetMobMaxCount))
        (if (<= (Variables|Default|GetMobsRemaining) 0)
          (CallFunction|TransitionEntered 5.0))
        (else
          (bind _mob_ (CallFunction|GetMobfromPool))
          (Default|AddMobtoQueue (.OutItem (Utilities|Array|Random (Variables|Default|GetMobSpawners))) _mob_))))))

(fn GetMobPoolSize
  (bind _values (Utilities|Map|Values (Variables|Default|GetMobsPool)))
  (for _array_element _values
    (LocalVariables|SetLocal%20Sum (+ (LocalVariables|GetLocal%20Sum) _array_element)))
  (return (LocalVariables|GetLocal%20Sum)))

(fn GetMobfromPool
  (return "/Game/MainGameFiles/Characters/Mobs/BP_Mob.BP_Mob_C"))