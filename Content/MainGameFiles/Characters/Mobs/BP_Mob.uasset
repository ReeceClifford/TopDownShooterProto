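; BP_Mob is an enemy character that constantly chases the player and dies from any damage.
; On BeginPlay it starts an AI MoveTo toward player 0, repeating two seconds after each completed move.
; Overlapping its Box with BP_MainCharacter reloads TopDownMap, resetting the level.
; Any damage destroys the actor immediately, with no health check, then calls CallOnDestroyed.
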(event OnComponentBeginOverlap(Box)
  (params (OverlappedComponent :type Primitive%20Component%20Object%20Reference) (OtherActor :type Actor%20Object%20Reference) (OtherComp :type Primitive%20Component%20Object%20Reference) (OtherBodyIndex :type Integer) (bFromSweep :type Boolean) (SweepResult :type Hit%20Result%20Structure%20%28by%20ref%29))
  ;[1 1 1] Reload Level / Reset on Impact
  (Utilities|Casting|CastToBP_MainCharacter OtherActor)
  (Game|OpenLevel(byObjectReference) "/Game/TopDown/Maps/TopDownMap.TopDownMap"))

(event Custom|Move
  ;[1 1 1] Enemies, Always Track Player
  (AI|AIMoveTo self "0, 0, 0" (Game|GetPlayerCharacter 0) 5.0 false :!label _label
    (:then
      (Utilities|FlowControl|Delay 2.0)
      (goto _label))))

(event EventBeginPlay
  ;[1 1 1] Start Enemy Movement
  (CallFunction|Move))

(event Game|Damage|EventAnyDamage
  (params (Damage :type Float%20%28single-precision%29) (DamageType :type Damage%20Type%20Object%20Reference) (InstigatedBy :type Controller%20Object%20Reference) (DamageCauser :type Actor%20Object%20Reference))
  ;[1 1 1] Manage Damage / Killing Mobs
  (Actor|DestroyActor)
  (Default|CallOnDestroyed))

(fn ConstructionScript)