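; BP_MobSpawner is a spawn point that releases queued mob classes one at a time at its own transform.
; AddMobToQueue spawns immediately if no mob overlaps its collision check, while looping timers keep calling SpawnMob without repeating that check.
; Each spawn binds to the mob's destroyed event, and OnMobDefeated forwards defeats to BP_MainGameMode.
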(event Custom|TryToSpawnMob
  (CallFunction|SpawnMob))

(event Custom|OnMobDefeated
  (bind _asbp_main_game_mode (Utilities|Casting|CastToBP_MainGameMode (Game|GetGameMode)))
  (Default|OnMobDefeated _asbp_main_game_mode))

(event EventBeginPlay
  (Utilities|Time|SetTimerbyEvent (delegate Custom|TryToSpawnMob) 2.0 true))

(fn ConstructionScript)

(fn AddMobtoQueue
  (params (MobClass :type BP%20Mob%20Class%20Reference%20%28by%20ref%29))
  ;[1 1 1] Add Mobs Left to Queue to be Spawned if is clear
  (Utilities|Array|Add (Variables|Default|GetMobQueue) MobClass)
  (if (not (Utilities|Array|IsValidIndex (Collision|GetOverlappingActors (Variables|Default|GetCollisionCheck) "/Game/MainGameFiles/Characters/Mobs/BP_Mob.BP_Mob_C" :!class /Script/Engine.PrimitiveComponent)))
    (CallFunction|SpawnMob)))

(fn SpawnMob
  ;[1 1 1] Spawn Mobs when Clear, in set position
  (if (Utilities|Array|IsValidIndex (Variables|Default|GetMobQueue))
    (bind _returnvalue (Game|SpawnActorfromClass (Utilities|Array|Get(acopy) (Variables|Default|GetMobQueue)) (Transformation|GetActorTransform) "AdjustIfPossibleButAlwaysSpawn" 0 0))
    (EventDispatchers|BindEventtoOnDestroyed _returnvalue (EventDispatchers|CreateEvent :!event Custom|OnMobDefeated))
    (Utilities|Array|RemoveIndex (Variables|Default|GetMobQueue))
    (Utilities|Time|SetTimerbyFunctionName 0 "SpawnMob" 1.5 true)
    (return true)
    (else
      (return false))))