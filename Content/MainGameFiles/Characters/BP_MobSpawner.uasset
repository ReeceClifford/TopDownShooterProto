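; Mob spawner actor that queues mob classes and spawns them at its own transform.
; AddMobToQueue appends a class and calls SpawnMob immediately if no BP_EnemyZombie overlaps its Sphere; otherwise the class just stays queued.
; SpawnMob spawns and removes the first queued entry, then sets a timer on itself to drain the queue every two seconds, without rechecking the overlap.
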(event EventBeginPlay)

(event Collision|EventActorBeginOverlap
  (params (OtherActor :type Actor%20Object%20Reference)))

(event EventTick
  (params (DeltaSeconds :type Float%20%28single-precision%29)))

(fn ConstructionScript)

(fn AddMobtoQueue
  (params (MobClass :type BP%20Enemy%20Zombie%20Class%20Reference%20%28by%20ref%29))
  (Utilities|Array|Add (Variables|Default|GetMobsInQueue) MobClass)
  (if (not (Utilities|Array|IsValidIndex (Collision|GetOverlappingActors (Variables|Default|GetSphere) "/Game/MainGameFiles/Characters/BP_EnemyZombie.BP_EnemyZombie_C" :!class /Script/Engine.PrimitiveComponent)))
    (CallFunction|SpawnMob)))

(fn SpawnMob
  (if (Utilities|Array|IsValidIndex (Variables|Default|GetMobsInQueue))
    (Game|SpawnActorfromClass (Utilities|Array|Get(acopy) (Variables|Default|GetMobsInQueue)) (Transformation|GetActorTransform) "Undefined" 0 0)
    (Utilities|Array|RemoveIndex (Variables|Default|GetMobsInQueue))
    (Utilities|Time|SetTimerbyFunctionName 0 "SpawnMob" 2.0)
    (return true)
    (else
      (return false))))