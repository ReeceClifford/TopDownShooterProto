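; BP_ShotgunProjectile is a shotgun shot that carries three pellets in one actor, each with its own overlap sphere.
; A pellet overlapping a BP_Mob applies DamageToDeal and destroys its paired sphere component, except the third, which destroys its own overlap sphere (Sphere5) rather than Sphere3.
; Overlapping anything else sets a five-second lifespan on the whole actor if that pellet's paired component is still valid.
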(event OnComponentBeginOverlap(Sphere1)
  (params (OverlappedComponent :type Primitive%20Component%20Object%20Reference) (OtherActor :type Actor%20Object%20Reference) (OtherComp :type Primitive%20Component%20Object%20Reference) (OtherBodyIndex :type Integer) (bFromSweep :type Boolean) (SweepResult :type Hit%20Result%20Structure%20%28by%20ref%29))
  (bind _sphere (Variables|Default|GetSphere))
  ;[1 1 1] Same as pistol, however 3 different collisions for 3 different bulltes
  (bind _asbp_mob (Utilities|Casting|CastToBP_Mob OtherActor)
    (:then
      (Game|Damage|ApplyDamage _asbp_mob (Variables|Default|GetDamageToDeal) 0 self)
      (Utilities|IsValid _sphere
        (:Is%20Valid
          (Components|DestroyComponent _sphere))))
    (:CastFailed
      (Utilities|IsValid (Variables|Default|GetSphere)
        (:Is%20Valid
          (Actor|SetLifeSpan 5.0))))))

(event OnComponentBeginOverlap(Sphere4)
  (params (OverlappedComponent :type Primitive%20Component%20Object%20Reference) (OtherActor :type Actor%20Object%20Reference) (OtherComp :type Primitive%20Component%20Object%20Reference) (OtherBodyIndex :type Integer) (bFromSweep :type Boolean) (SweepResult :type Hit%20Result%20Structure%20%28by%20ref%29))
  (bind _sphere2 (Variables|Default|GetSphere2))
  ;[1 1 1] Same as pistol, however 3 different collisions for 3 different bulltes
  (bind _asbp_mob (Utilities|Casting|CastToBP_Mob OtherActor)
    (:then
      (Game|Damage|ApplyDamage _asbp_mob (Variables|Default|GetDamageToDeal) 0 self)
      (Utilities|IsValid _sphere2
        (:Is%20Valid
          (Components|DestroyComponent _sphere2))))
    (:CastFailed
      (Utilities|IsValid (Variables|Default|GetSphere2)
        (:Is%20Valid
          (Actor|SetLifeSpan 5.0))))))

(event OnComponentBeginOverlap(Sphere5)
  (params (OverlappedComponent :type Primitive%20Component%20Object%20Reference) (OtherActor :type Actor%20Object%20Reference) (OtherComp :type Primitive%20Component%20Object%20Reference) (OtherBodyIndex :type Integer) (bFromSweep :type Boolean) (SweepResult :type Hit%20Result%20Structure%20%28by%20ref%29))
  (bind _sphere5 (Variables|Default|GetSphere5))
  ;[1 1 1] Same as pistol, however 3 different collisions for 3 different bulltes
  (bind _asbp_mob (Utilities|Casting|CastToBP_Mob OtherActor)
    (:then
      (Game|Damage|ApplyDamage _asbp_mob (Variables|Default|GetDamageToDeal) 0 self)
      (Utilities|IsValid _sphere5
        (:Is%20Valid
          (Components|DestroyComponent _sphere5))))
    (:CastFailed
      (Utilities|IsValid (Variables|Default|GetSphere3)
        (:Is%20Valid
          (Actor|SetLifeSpan 5.0))))))

(fn ConstructionScript)