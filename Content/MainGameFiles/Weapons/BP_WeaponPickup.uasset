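; BP_WeaponPickup is a weapon pickup that swaps the main character's current weapon when touched.
; On BeginPlay it sets its Niagara effect to the shotgun system if WeaponToSwapTo is the shotgun projectile class, otherwise to the sniper system.
; Sphere overlap by BP_MainCharacter copies the weapon and magazine values onto the character, then hides the pickup without destroying it or disabling its collision.
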(event OnComponentBeginOverlap(Sphere)
  (params (OverlappedComponent :type Primitive%20Component%20Object%20Reference) (OtherActor :type Actor%20Object%20Reference) (OtherComp :type Primitive%20Component%20Object%20Reference) (OtherBodyIndex :type Integer) (bFromSweep :type Boolean) (SweepResult :type Hit%20Result%20Structure%20%28by%20ref%29))
  (bind _asbp_main_character (Utilities|Casting|CastToBP_MainCharacter OtherActor))
  (Variables|/Game/MainGameFiles/Characters/MainCharacter/BP_MainCharacter.BP_MainCharacter_C|SetCurrentWeapon _asbp_main_character (Variables|Default|GetWeaponToSwapTo))
  (Variables|/Game/MainGameFiles/Characters/MainCharacter/BP_MainCharacter.BP_MainCharacter_C|SetCurrentWeaponMag _asbp_main_character (Variables|Default|GetWeaponPickUpMag))
  (Rendering|SetActorHiddenInGame self true))

(event EventBeginPlay
  (bind _niagara (Variables|Default|GetNiagara))
  (if (== (Variables|Default|GetWeaponToSwapTo) "/Game/MainGameFiles/Weapons/BP_ShotgunProjectile.BP_ShotgunProjectile_C")
    (Class|NiagaraComponent|SetAsset _niagara "/Game/MainGameFiles/Materials/NS_Shotgun.NS_Shotgun" true)
    (else
      (Class|NiagaraComponent|SetAsset _niagara "/Game/MainGameFiles/Materials/NS_Sniper.NS_Sniper" true))))

(fn ConstructionScript)